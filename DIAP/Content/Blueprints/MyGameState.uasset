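; Game state for a multiplayer elimination game in which a timed raffle randomly afflicts players and kills those still afflicted at the next draw.
; Tick moves the match from waiting for players through ready-up to a countdown, after which play begins.
; Each raffle kills, checks for a lone winner or no survivors, then re-afflicts and reschedules while play continues.
; The state's RepNotify swaps local UI screens and enables character movement.
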(event Custom|Start%20Playing
  ;[1 1 1] Start Playing
  (Variables|Default|SetCurrent%20Game%20State "NewEnumerator1")
  (CallFunction|Raffle))

(event Custom|KillAfflicted
  (if (Utilities|Enum|Equal(Enum) (Variables|Default|GetCurrent%20Game%20State) "NewEnumerator1")
    (for (_array_element _array_index) (Variables|Default|GetPlayerArray)
      (bind _asmy_player_state (Utilities|Casting|CastToMyPlayerState _array_element))
      (if (Variables|/Game/Blueprints/MyPlayerState.MyPlayerState_C|GetisAfflicted _asmy_player_state)
        (Default|MakeCharacterDie _asmy_player_state _array_index)))))

(event Custom|Raffle
  ;[1 1 1] Raffle
  (CallFunction|KillAfflicted)
  (CallFunction|CheckifGameOver)
  (if (Utilities|Enum|Equal(Enum) (Variables|Default|GetCurrent%20Game%20State) "NewEnumerator1")
    (for _index (range 0 (Variables|Default|GetNumberOf%20Afllicted%20Players))
      (bind _asmy_player_state (Utilities|Casting|CastToMyPlayerState (Utilities|Array|Get(acopy) (Variables|Default|GetPlayerArray) (Math|Random|RandomIntegerinRange 1 (Utilities|Array|Length (Variables|Default|GetPlayerArray))))))
      (Default|MakeAfflicted _asmy_player_state))
    (if (Utilities|Enum|Equal(Enum) (Variables|Default|GetCurrent%20Game%20State) "NewEnumerator1")
      (bind _returnvalue (Utilities|Time|SetTimerbyFunctionName 0 "Raffle" (Variables|Default|GetTimeToNextRaffle)))
      (Variables|Default|SetCountDownTimer _returnvalue))
    (else
      (Class|KismetSystemLibrary|ClearTimerHandle (Variables|Default|GetCountDownTimer)))))

(event Custom|Start%20Raffle
  ;[1 1 1] Raffle
  (bind _returnvalue (Utilities|Time|SetTimerbyFunctionName 0 "Start Playing" (Variables|Default|GetRaffle%20Delay%20in%20Seconds)))
  (Variables|Default|SetCountDownTimer _returnvalue))

(event Custom|Check%20If%20Game%20Over
  (Variables|Default|SetNumberOfAlivePlayers 0)
  (for _array_element (Variables|Default|GetPlayerArray)
    (bind _asmy_player_state (Utilities|Casting|CastToMyPlayerState _array_element))
    (if (Variables|/Game/Blueprints/MyPlayerState.MyPlayerState_C|GetIsAlive _asmy_player_state)
      (Math|Integer|IncrementInt (Variables|Default|GetNumberOfAlivePlayers))))
  (Utilities|FlowControl|Sequence
    (:then_0
      (if (== (Variables|Default|GetNumberOfAlivePlayers) 0)
        (Variables|Default|SetCurrent%20Game%20State "NewEnumerator5")))
    (:then_1
      (if (== (Variables|Default|GetNumberOfAlivePlayers) 1)
        (bind _array_element_2 (Utilities|Array|ForEachLoopwithBreak (Variables|Default|GetPlayerArray) :!label _label)
          (:LoopBody
            (bind _asmy_player_state_2 (Utilities|Casting|CastToMyPlayerState _array_element_2))
            (if (Math|Boolean|Equal(Boolean) (Variables|/Game/Blueprints/MyPlayerState.MyPlayerState_C|GetIsAlive _asmy_player_state_2) true)
              (Default|MakeIsWinner _asmy_player_state_2)
              (goto _label Break)))
          (:Completed
            (Variables|Default|SetCurrent%20Game%20State "NewEnumerator4")))))))

(event EventBeginPlay
  (Variables|Default|SetCurrent%20Game%20State "NewEnumerator0"))

(event EventTick
  (params (DeltaSeconds :type Float%20%28single-precision%29))
  (bind _playerarray (Variables|Default|GetPlayerArray))
  (bind _returnvalue (Utilities|Array|Length _playerarray))
  (Utilities|FlowControl|Sequence
    (:then_0
      (if (Utilities|Enum|Equal(Enum) (Variables|Default|GetCurrent%20Game%20State) "NewEnumerator0")
        (Variables|Default|SetCurNumberOfPlayers _returnvalue)
        (if (>= _returnvalue (Variables|Default|GetMinPlayersToStart))
          (Variables|Default|SetCurrent%20Game%20State "NewEnumerator2"))))
    (:then_1
      (if (Utilities|Enum|Equal(Enum) (Variables|Default|GetCurrent%20Game%20State) "NewEnumerator2")
        (if (CallFunction|AllIsReady)
          (Variables|Default|SetCurrent%20Game%20State "NewEnumerator3")
          (CallFunction|StartRaffle)
          (Development|PrintString "true"))))))

(fn ConstructionScript)

(fn OnRepGameStartTimer)

(fn OnRepRandomTimerValue1)

(fn OnRepCurrentGameState
  (switch Utilities|FlowControl|Switch|SwitchonGameStates (Variables|Default|GetCurrent%20Game%20State)
    (:NewEnumerator2
      (bind _asmy_player_controller (Utilities|Casting|CastToMyPlayerController (Game|GetPlayerController 0)))
      (Default|RemoveWaitingforPlayers _asmy_player_controller)
      (Default|ShowWaitingtoReadyUp _asmy_player_controller))
    (:NewEnumerator3
      (bind _asmy_player_controller_2 (Utilities|Casting|CastToMyPlayerController (Game|GetPlayerController 0)))
      (Default|RemoveWaitingtoReadyUp _asmy_player_controller_2)
      (Default|ShowRaffleCountdown _asmy_player_controller_2))
    (:NewEnumerator1
      (bind _asmy_player_controller_3 (Utilities|Casting|CastToMyPlayerController (Game|GetPlayerController 0)))
      (Default|RemoveRaffleCountdown _asmy_player_controller_3)
      (bind _asfirst_person_character (Utilities|Casting|CastToFirstPersonCharacter (Game|GetPlayerCharacter 0)))
      (Variables|/Game/FirstPersonBP/Blueprints/FirstPersonCharacter.FirstPersonCharacter_C|SetCanMove _asfirst_person_character true))
    (:NewEnumerator4
      (bind _asmy_player_controller_4 (Utilities|Casting|CastToMyPlayerController (Game|GetPlayerController 0) :!label _label))
      (Default|ShowGameOver _asmy_player_controller_4))
    (:NewEnumerator5
      (goto _label))))

(fn AllIsReady
  (LocalVariables|SetLocal%20Ready true)
  (bind _array_element (Utilities|Array|ForEachLoopwithBreak (Variables|Default|GetPlayerArray) :!label _label)
    (:LoopBody
      (bind _asmy_player_state (Utilities|Casting|CastToMyPlayerState _array_element))
      (if (Math|Boolean|Equal(Boolean) (Variables|/Game/Blueprints/MyPlayerState.MyPlayerState_C|GetReady _asmy_player_state) false)
        (LocalVariables|SetLocal%20Ready false)
        (goto _label Break)))
    (:Completed
      (Development|PrintString "rep notifiy")
      (return (LocalVariables|GetLocal%20Ready)))))