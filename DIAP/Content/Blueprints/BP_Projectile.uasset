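; Networked projectile that passes an affliction from its owning character to the FirstPersonCharacter it hits.
; On hit it plays an attenuated sound with randomized pitch, then branches on authority.
; The authority afflicts a hit character, clears the affliction on the owner, and destroys the projectile whatever it struck.
; Remote instances only add an impact particle effect at the hit location.
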(event `self.ReceiveHit`
  (params (MyComp :type "PrimitiveComponent Object Reference") (Other :type "Actor Object Reference") (OtherComp :type "PrimitiveComponent Object Reference") (bSelfMoved :type Boolean) (HitLocation :type "Vector Structure") (HitNormal :type "Vector Structure") (NormalImpulse :type "Vector Structure") (Hit :type "HitResult Structure (by ref)"))
  ;[0 1 0] Sound
  (`GameplayStatics.PlaySoundAtLocation` "/Game/Sounds/SoundCue_Attentuated.SoundCue_Attentuated" HitLocation (struct) (`self.VolumeMultiplier`) (`KismetMathLibrary.RandomFloatInRange` 0.8 1.2))
  (`/Engine/EditorBlueprintResources/ActorMacros.Switch Has Authority`
    (:`Authority`
      ;[1 1 1] Hit Character
      (`|ExecutionSequence`
        (:`then_0`
          (bind _asfirst_person_character (cast `/Game/FirstPersonBP/Blueprints/FirstPersonCharacter` Other))
          (`/Game/FirstPersonBP/Blueprints/FirstPersonCharacter.Afflict Interface` _asfirst_person_character)
          (bind _asfirst_person_character_2 (cast `/Game/FirstPersonBP/Blueprints/FirstPersonCharacter` (`self.GetOwner`)))
          (`/Game/FirstPersonBP/Blueprints/FirstPersonCharacter.Undo Affliction Interface` _asfirst_person_character_2))
        (:`then_1`
          (`self.K2_DestroyActor`))))
    (:`Remote`
      (`GameplayStatics.SpawnEmitterAtLocation` "/Game/Effects/P_Hit.P_Hit" HitLocation))))

(fn `UserConstructionScript`)